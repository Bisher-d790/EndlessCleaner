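; Germ pickup that plays a collection effect when an ECCharacter overlaps its collision.
; The Scaledown timeline drives the mesh's scale, then after a short delay the actor detaches and hides the mesh rather than being destroyed.
; When DrawDebugSpheres is on, Tick draws spheres at the WaypointMovementComponent's waypoints and, if beacon movement is enabled, at the beacon position.
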(event OnComponentBeginOverlap(Collision)
  (params (OverlappedComponent :type Primitive%20Component%20Object%20Reference) (OtherActor :type Actor%20Object%20Reference) (OtherComp :type Primitive%20Component%20Object%20Reference) (OtherBodyIndex :type Integer) (bFromSweep :type Boolean) (SweepResult :type Hit%20Result%20Structure%20%28by%20ref%29))
  ;[1 1 1] On Collected FX
  (Utilities|Casting|CastToECCharacter OtherActor)
  (bind _scalefloat (Timeline|Scaledown PlayFromStart)
    (:Update
      (Transformation|SetWorldScale3D (Variables|Character|GetMesh) (Math|Conversions|ToVector(Float) _scalefloat)))
    (:Finished
      (Utilities|FlowControl|Delay 0.2)
      (Transformation|DetachFromActor "KeepRelative" "KeepRelative" "KeepRelative")
      (Rendering|SetVisibility (Variables|Character|GetMesh) false false))))

(event EventTick
  (params (DeltaSeconds :type Float%20%28single-precision%29))
  (if (Variables|Default|GetbDrawDebugSpheres)
    ;[1 1 1] Draw Debug Spheres
    (bind _aswaypoint_movement_component (Utilities|Casting|CastToWaypointMovementComponent (Variables|Default|GetMovementComponent)))
    (for _array_element (Variables|/Script/EndlessCleaner.WaypointMovementComponent|GetWaypointLocations _aswaypoint_movement_component)
      (Rendering|Debug|DrawDebugSphere _array_element 5e+01 12 "(R=1.000000,G=0.068094,B=0.000000,A=1.000000)" 0.0)
      (if (Variables|/Script/EndlessCleaner.WaypointMovementComponent|GetbUseBeaconForMovement _aswaypoint_movement_component)
        (bind _returnvalue (Class|WaypointMovementComponent|GetBeaconPosition _aswaypoint_movement_component))
        (Rendering|Debug|DrawDebugSphere _returnvalue 5e+01 12 "(R=0.000000,G=0.142265,B=1.000000,A=1.000000)" 0.0)))))

(fn ConstructionScript)